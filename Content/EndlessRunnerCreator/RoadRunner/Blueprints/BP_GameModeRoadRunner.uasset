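; Game mode for the Road Runner endless runner that keeps a persistent best score.
; On BeginPlay it loads save slot "1" and copies the stored Xp into Resw.
; The record event replaces Resw when given a higher value and writes it back to that slot.
; Saving uses its own Seve object, created when none is valid, rather than the loaded one.
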(event `self.ReceiveBeginPlay`
  (`parent.ReceiveBeginPlay`)
  (bind _returnvalue (`GameplayStatics.LoadGameFromSlot` "1"))
  (bind _asseve (cast `/Game/EndlessRunnerCreator/RoadRunner/Blueprints/seve` _returnvalue))
  (set `self.resw` (`/Game/EndlessRunnerCreator/RoadRunner/Blueprints/seve.xp` _asseve)))

(event `record`
  (params (NewParam :type Integer))
  (if (> NewParam (`self.resw`))
    (bind _output_get (set `self.resw` NewParam))
    (`self.NewVar_0`
      (:`then`
        _)
      (:`else`
        (bind _returnvalue (`GameplayStatics.CreateSaveGameObject` "/Game/EndlessRunnerCreator/RoadRunner/Blueprints/seve.seve_C"))
        (set `self.NewVar_0` _returnvalue)))
    (set `/Game/EndlessRunnerCreator/RoadRunner/Blueprints/seve.xp` _output_get (`self.NewVar_0`))
    (`GameplayStatics.SaveGameToSlot` (`self.NewVar_0`) "1")))

(fn `UserConstructionScript`
  (`parent.UserConstructionScript`))