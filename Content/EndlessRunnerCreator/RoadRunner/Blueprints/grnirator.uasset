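; Self-replicating track segment for the Road Runner endless runner, which places its tree at a random world X on BeginPlay.
; When the player overlaps Box, it spawns the next Grnirator at its Arrow's transform.
; Overlapping Box1 adds XP to the player, calls Sdf on the player's Vd reference, then destroys the segment after a short delay.
; Both triggers are guarded by DoOnce.
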(event `self.ReceiveBeginPlay`
  (`SceneComponent.K2_SetWorldLocation` (`self.Leave-Tree-01a`) (`KismetMathLibrary.MakeVector` (`KismetMathLibrary.RandomFloatInRange` -1000.0 1000.0)) false false))

(event `self.Box.OnComponentBeginOverlap`
  (params (OverlappedComponent :type "PrimitiveComponent Object Reference") (OtherActor :type "Actor Object Reference") (OtherComp :type "PrimitiveComponent Object Reference") (OtherBodyIndex :type Integer) (bFromSweep :type Boolean) (SweepResult :type "HitResult Structure (by ref)"))
  (cast `/Game/EndlessRunnerCreator/RoadRunner/Blueprints/BP_PlayerRoadRunner` OtherActor)
  (`/Engine/EditorBlueprintResources/StandardMacros.DoOnce` false
    (:`Completed`
      (`|SpawnActorFromClass` "grnirator_C" (`SceneComponent.K2_GetComponentToWorld` (`self.Arrow`)) "Undefined" "OverrideRootScale" null null))))

(event `self.Box1.OnComponentBeginOverlap`
  (params (OverlappedComponent :type "PrimitiveComponent Object Reference") (OtherActor :type "Actor Object Reference") (OtherComp :type "PrimitiveComponent Object Reference") (OtherBodyIndex :type Integer) (bFromSweep :type Boolean) (SweepResult :type "HitResult Structure (by ref)"))
  (bind _asbp_player_road_runner (cast `/Game/EndlessRunnerCreator/RoadRunner/Blueprints/BP_PlayerRoadRunner` OtherActor))
  (`/Engine/EditorBlueprintResources/StandardMacros.DoOnce` false
    (:`Completed`
      (bind _output_get (set `/Game/EndlessRunnerCreator/RoadRunner/Blueprints/BP_PlayerRoadRunner.Xp` (+ (stale _output_get) 100) _asbp_player_road_runner))
      (`/Game/EndlessRunnerCreator/RoadRunner/Blueprints/hud.sdf` (`/Game/EndlessRunnerCreator/RoadRunner/Blueprints/BP_PlayerRoadRunner.vd` _asbp_player_road_runner))
      (`KismetSystemLibrary.Delay` 0.2)
      (`self.K2_DestroyActor`))))

(fn `UserConstructionScript`)