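; Gold pickup actor for the RoadRunner game that adds one to the player's Gold when touched.
; On BeginPlay a Timeline yaws its Fish component through a 0–360 degree lerp, while a delay destroys the actor after five seconds if not collected.
; A BP_PlayerRoadRunner overlapping the Sphere gets the gold and activates the NSPickupCurrency effect, then the actor is destroyed after a short delay.
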(event `self.ReceiveBeginPlay`
  (`|ExecutionSequence`
    (:`then_0`
      (bind (_direction _newtrack_0) (`Timeline|Timeline_0` :!via `PlayFromStart`)
        (:`Update`
          (`SceneComponent.K2_SetWorldRotation` (`self.fish`) (`KismetMathLibrary.MakeRotator` 0.0 0.0 (`KismetMathLibrary.Lerp` 0.0 360.0 _newtrack_0)) false false))))
    (:`then_1`
      (`KismetSystemLibrary.Delay` 5.0)
      (`self.K2_DestroyActor` :!label _label))))

(event `self.Sphere.OnComponentBeginOverlap`
  (params (OverlappedComponent :type "PrimitiveComponent Object Reference") (OtherActor :type "Actor Object Reference") (OtherComp :type "PrimitiveComponent Object Reference") (OtherBodyIndex :type Integer) (bFromSweep :type Boolean) (SweepResult :type "HitResult Structure (by ref)"))
  (bind _asbp_player_road_runner (cast `/Game/EndlessRunnerCreator/RoadRunner/Blueprints/BP_PlayerRoadRunner` OtherActor))
  (bind _output_get (set `/Game/EndlessRunnerCreator/RoadRunner/Blueprints/BP_PlayerRoadRunner.gold` (+ (stale _output_get) 1) _asbp_player_road_runner))
  (`ActorComponent.Activate` (`self.NS_PickupCurrency`) true)
  (`KismetSystemLibrary.Delay` 0.5)
  (goto _label))

(fn `UserConstructionScript`)